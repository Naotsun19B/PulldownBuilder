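; Test pulldown list generator that builds dropdown rows procedurally from a struct instance.
; It reads a base name and row count from the struct container, then creates numbered "RowName_Index" entries labeled Even or Odd.
; Each tooltip shows the first outer object, or "None" if absent.
; A second override returns the FilterPulldownStructTypes variable as the generator's struct type filter.
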(fn `GetFilterPulldownStructTypesFromBlueprint`
  (returns (ReturnValue :type "Array of Name"))
  (locals (FilterPulldownStructTypes :type "Array of Name"))
  (return (`local.FilterPulldownStructTypes`)))

(fn `GetPulldownRowsFromBlueprint`
  (params (OuterObjects :type "Array of Object Object Reference (by ref)") (StructInstance :type "StructContainer Structure (by ref)"))
  (returns (ReturnValue :type "Array of PulldownRow Structure"))
  (locals (PulldownRows :type "Array of PulldownRow Structure"))
  (bind (_structdata _returnvalue) (`|Get_StructContainer` StructInstance))
  (bind (_numofrows _rowname) (break `TestPulldown4` _structdata))
  (if _returnvalue
    (for _index (range 1 (+ _numofrows 1))
      (bind _result (`|FormatText` "{0}_{1}" (`KismetTextLibrary.Conv_StringToText` (`KismetStringLibrary.Conv_NameToString` _rowname)) _index))
      (`KismetArrayLibrary.Array_Add` (`local.PulldownRows`) (make `PulldownRow` (`KismetTextLibrary.Conv_TextToString` _result) (`|FormatText` "{0} ({1})" _result (`KismetMathLibrary.SelectString` "Even" "Odd" (== (mod _index 2) 0))) (select `bool` (`KismetArrayLibrary.Array_IsValidIndex` OuterObjects) :`false` "None" :`true` (`KismetTextLibrary.Conv_ObjectToText` (`|GetArrayItem` OuterObjects)))))))
  (return (`local.PulldownRows`)))